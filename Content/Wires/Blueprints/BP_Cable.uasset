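; Spline-based cable actor that visually fills with power over time and drains when filling stops.
; The construction script builds two overlapping spline meshes per segment, storing only the collision-disabled one for material updates.
; Tick moves Distance at FillSpeed while IsFilling, setting IsPowered at half the spline length and clearing it when filling stops.
; Each tick, EPowerCable converts Distance into a per-segment "Percentage" material parameter to show the fill.
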(event `self.ReceiveTick`
  (params (DeltaSeconds :type "Float (single-precision)"))
  (bind _returnvalue (* (`SplineComponent.GetSplineLength` (`self.Spline`)) 0.5))
  (`|ExecutionSequence`
    (:`then_0`
      (if (`self.bIsFilling`)
        (bind _output_get (set `self.Distance` (`KismetMathLibrary.FClamp` (+ (* DeltaSeconds (`self.FillSpeed`)) (`self.Distance`)) 0.0 _returnvalue)))
        (if (and (>= _output_get _returnvalue) (not (`self.bIsPowered`)))
          (set `self.bIsPowered` true))
        (else
          (set `self.Distance` (`KismetMathLibrary.FClamp` (- (`self.Distance`) (* DeltaSeconds (`self.FillSpeed`))) 0.0 _returnvalue))
          (if (`self.bIsPowered`)
            (set `self.bIsPowered` false)))))
    (:`then_1`
      (`self.ePowerCable`))))

(event `ePowerCable`
  (bind _returnvalue (`SplineComponent.GetDistanceAlongSplineAtSplinePoint` (`self.Spline`) (- (`self.CurrentIndex`) 1)))
  (bind _output (`|GetArrayItem` (`self.Components`) (- (`self.CurrentIndex`) 1)))
  (for _index (range (`SplineComponent.GetNumberOfSplinePoints` (`self.Spline`)))
    (set `self.CurrentIndex` _index)
    (if (< (`SplineComponent.GetDistanceAlongSplineAtSplinePoint` (`self.Spline`) (`self.CurrentIndex`)) (`self.Distance`))
      (`/Engine/EditorBlueprintResources/StandardMacros.IsValid` _output
        (:`Is Valid`
          (`MeshComponent.SetScalarParameterValueOnMaterials` _output "Percentage" -1.0)))
      (else
        (`/Engine/EditorBlueprintResources/StandardMacros.IsValid` _output
          (:`Is Valid`
            (`MeshComponent.SetScalarParameterValueOnMaterials` _output "Percentage" (`KismetMathLibrary.FClamp` (* (- (* (/ (- (`self.Distance`) (* _returnvalue 0.5)) (- (`SplineComponent.GetDistanceAlongSplineAtSplinePoint` (`self.Spline`) (`self.CurrentIndex`)) _returnvalue)) 2.0) 1.0) -1.0) -1.0))))))))

(fn `UserConstructionScript`
  (bind _spline (`self.Spline`))
  (for _index (range (+ (- (`SplineComponent.GetNumberOfSplinePoints` (`self.Spline`)) 2) 1))
    (bind _returnvalue (`AddComponent|NODE_AddSplineMeshComponent-0`))
    (`PrimitiveComponent.SetCollisionEnabled` _returnvalue "NoCollision")
    (`KismetArrayLibrary.Array_Add` (`self.Components`) _returnvalue)
    (`SceneComponent.K2_AttachToComponent` _returnvalue (`self.DefaultSceneRoot`) "None" "KeepRelative" "KeepRelative" "KeepRelative" true)
    (bind (_location _tangent) (`SplineComponent.GetLocationAndTangentAtSplinePoint` _spline _index "Local"))
    (bind (_location_2 _tangent_2) (`SplineComponent.GetLocationAndTangentAtSplinePoint` _spline (+ _index 1) "Local"))
    (`SplineMeshComponent.SetStartAndEnd` _returnvalue _location _tangent _location_2 _tangent_2 true)
    (bind _returnvalue_2 (`AddComponent|NODE_AddSplineMeshComponent-1`))
    (`SceneComponent.K2_AttachToComponent` _returnvalue_2 (`self.DefaultSceneRoot`) "None" "KeepRelative" "KeepRelative" "KeepRelative" true)
    (`SplineMeshComponent.SetStartAndEnd` _returnvalue_2 _location _tangent _location_2 _tangent_2 true)))